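; Enemy summon ability that spawns random minions at a set of locations, using the shaman's summon montage.
; On activation it shuffles the spawn locations, plays a ground Niagara effect at each, then starts the montage and waits for its attack gameplay event.
; That event starts a delayed loop that spawns one minion per location in quick succession.
; Minions are raised by capsule half-height and face along the direction from summoner to spawn point.
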(event `self.K2_ActivateAbility`
  (bind _returnvalue (`self.GetSpawnLocations`))
  (bind _output_get (set `self.SpawnLocations` _returnvalue))
  (`KismetArrayLibrary.Array_Shuffle` _output_get) ; Randomizing array elements so spawn locations are random and not index 0 to array length
  (for _array_element _output_get
    (`NiagaraFunctionLibrary.SpawnSystemAtLocation` "/Game/Assets/Effects/Combat/NS_GroundSummon.NS_GroundSummon" _array_element))
  (`AbilityTask_PlayMontageAndWait.CreatePlayMontageAndWaitProxy` "None" "/Game/Assets/Enemies/Shaman/Animations/AM_Shaman_Summon.AM_Shaman_Summon"
    (:`then`
      (`AbilityTask_WaitGameplayEvent.WaitGameplayEvent` (struct :`TagName` "Montage.Attack.1") null
        (:`EventReceived`
          (if (< (`self.SpawnLocationIndex`) (`KismetArrayLibrary.Array_Length` (`self.SpawnLocations`))) :!label _label
            (`self.SpawnMinion`)
            (`/Engine/EditorBlueprintResources/StandardMacros.IncrementInt` (`self.SpawnLocationIndex`)
              (:`  `
                (`KismetSystemLibrary.Delay` 0.2)
                (goto _label)))))))))

(fn `SpawnMinion`
  (returns (SpawnedMinion :type "ASCharacterBase Object Reference"))
  (bind _returnvalue (`self.GetRandomMinionClassCDO`))
  (bind _output (`|GetArrayItem` (`self.SpawnLocations`) (`self.SpawnLocationIndex`)))
  (bind _returnvalue_2 (`|SpawnActorFromClass` (`GameplayStatics.GetObjectClass` _returnvalue) (`KismetMathLibrary.MakeTransform` (+ _output (`KismetMathLibrary.MakeVector` 0.0 0.0 (`CapsuleComponent.GetScaledCapsuleHalfHeight` (`Character.CapsuleComponent` _returnvalue)))) (`KismetMathLibrary.FindLookAtRotation` (`Actor.K2_GetActorLocation` (`self.GetAvatarActorFromActorInfo`)) _output)) "AdjustIfPossibleButDontSpawnIfColliding" "MultiplyWithRoot" null null))
  (return _returnvalue_2))